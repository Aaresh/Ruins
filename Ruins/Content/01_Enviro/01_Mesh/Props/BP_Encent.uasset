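; Incense prop Blueprint with an optional cover and an optional effect, configured entirely in the construction script.
; The COVER and VFX flags, when off, destroy the EncensTop and NSEncent components respectively.
; The script then sets NSEncent to a random uniform integer world scale, re-rolled on each construction run, without checking whether VFX removed it.
; The event graph has no active logic.
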(event EventBeginPlay)

(event Collision|EventActorBeginOverlap
  (params (OtherActor :type Actor%20Object%20Reference)))

(event EventTick
  (params (DeltaSeconds :type Float%20%28single-precision%29)))

(fn ConstructionScript
  (Utilities|FlowControl|Sequence
    (:then_0
      (if (not (Variables|Default|GetCOVER))
        (Components|DestroyComponent (Variables|Default|GetEncens_Top))))
    (:then_1
      (if (not (Variables|Default|GetVFX))
        (Components|DestroyComponent (Variables|Default|GetNS_Encent))))
    (:then_2
      (Transformation|SetWorldScale3D (Variables|Default|GetNS_Encent) (Math|Conversions|ToVector(Float) (Math|Random|RandomIntegerinRange 3 8))))))